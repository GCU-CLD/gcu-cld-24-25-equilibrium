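; Switchable electric fence hazard that spans from the actor's origin to an EndPoint.
; The construction script stretches and aims a hidden HazardMesh along that span and passes the endpoint to the particle system.
; Switch events call the parent's on/off logic and toggle particles and sound, with InvertBehaviour swapping them.
; SetInitialStatus routes through these events, resolving to on for either status value.
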(event `/Game/PGTemplate/Blueprints/Objects/Switches/Core/SwitchInterface.SwitchOn`
  (bind _particlesystem (`self.ParticleSystem`))
  (bind _sound (`self.Sound`))
  (if (`self.InvertBehaviour`)
    (`parent.SwitchOff` :!label _label)
    (`ActorComponent.Deactivate` _particlesystem)
    (`AudioComponent.Stop` _sound)
    (else
      (`parent.SwitchOn` :!label _label_2)
      (`ActorComponent.Activate` _particlesystem false)
      (`AudioComponent.Play` _sound 0.0))))

(event `/Game/PGTemplate/Blueprints/Objects/Switches/Core/SwitchInterface.SwitchOff`
  (if (`self.InvertBehaviour`)
    (goto _label_2)
    (else
      (goto _label))))

(event `/Game/PGTemplate/Blueprints/Objects/Switches/Core/SwitchInterface.SetInitialStatus`
  (params (InitialStatus :type Boolean))
  (bind _invertbehaviour (`self.InvertBehaviour`))
  (if InitialStatus
    (if _invertbehaviour
      (`self.SwitchOff` :!label _label_3)
      (else
        (`self.SwitchOn` :!label _label_4)))
    (elif _invertbehaviour
      (goto _label_3)
      (else
        (goto _label_4)))))

(fn `UserConstructionScript`
  (bind _endpoint (`self.EndPoint`))
  (bind _hazardmesh (`self.HazardMesh`))
  (`SceneComponent.K2_SetRelativeLocation` _hazardmesh (/ _endpoint 2.0) false false)
  (`SceneComponent.K2_SetRelativeRotation` _hazardmesh (`KismetMathLibrary.FindLookAtRotation` (0.0 0.0 0.0) _endpoint) false false)
  (`SceneComponent.SetRelativeScale3D` _hazardmesh (`KismetMathLibrary.MakeVector` (* (`KismetMathLibrary.VSize` _endpoint) 0.01) 0.6 0.1))
  (`SceneComponent.K2_SetRelativeLocation` (`self.End`) (`self.EndPoint`) false false)
  (`parent.UserConstructionScript`)
  (`SceneComponent.SetVisibility` (`self.HazardMesh`) false false)
  (`NiagaraComponent.SetVariableVec3` (`self.ParticleSystem`) "EndPosition" (`self.EndPoint`)))