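; Rocket projectile hazard that damages the platform game character and explodes on overlap with any actor except its instigator.
; A character hit passes damage and the reversed forward vector to RegisterHit, then plays a hit montage if none is active.
; Impacts spawn a Niagara effect and sound before destroying the rocket.
; It also expires after its lifespan, and OnReset destroys it without impact effects.
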(event `self.ReceiveBeginPlay`
  (`self.SetLifeSpan` (`self.Lifespan`)))

(event `self.ReceiveActorBeginOverlap`
  (params (OtherActor :type "Actor Object Reference"))
  (bind _returnvalue (`self.K2_GetActorLocation`))
  (if (!= OtherActor (`self.InstigatingActor`))
    (bind _asbp_platform_game_character (cast `/Game/PGTemplate/Blueprints/Characters/Core/BP_PlatformGameCharacter` OtherActor)
      (:`then`
        (`/Game/PGTemplate/Blueprints/Characters/Core/BP_PlatformGameCharacter.RegisterHit` _asbp_platform_game_character (* (`self.GetActorForwardVector`) -1.0) (`self.K2_GetActorLocation`) (`self.DamageDone`))
        (`/Engine/EditorBlueprintResources/StandardMacros.IsValid` (`Character.GetCurrentMontage` _asbp_platform_game_character)
          (:`Is Valid`
            _)
          (:`Is Not Valid`
            (`|PlayMontage` (`Character.Mesh` _asbp_platform_game_character) "/Game/PGTemplate/Blueprints/Characters/Core/Animations/Custom/HitAnim_Anim_Montage.HitAnim_Anim_Montage"
              (:`then`
                _)))))
      (:`CastFailed`
        _))
    (`NiagaraFunctionLibrary.SpawnSystemAtLocation` "/Game/PGTemplate/Blueprints/Objects/Hazards/VFX/RocketImpact_NS.RocketImpact_NS" _returnvalue)
    (`GameplayStatics.PlaySoundAtLocation` "/Game/PGTemplate/Blueprints/Objects/Hazards/Audio/MissileHit.MissileHit" _returnvalue (struct) 1.0 1.0 0.0 null null null null)
    (`self.K2_DestroyActor` :!label _label)))

(event `self.K2_OnReset`
  (goto _label))

(fn `UserConstructionScript`)